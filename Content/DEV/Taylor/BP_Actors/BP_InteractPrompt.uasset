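; BP_InteractPrompt is an interaction prompt actor that displays a button prompt and function label through a WI_Interact widget component.
; On BeginPlay it hides the widget's texts and image, then fills the texts from its Prompt and Func variables.
; ShowPrompt and HidePrompt play and reverse one Timeline that fades those elements' opacity.
; The actor has no active trigger logic of its own, as its overlap and tick events are empty.
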(event Custom|ShowPrompt
  (bind _aswi_interact (Utilities|Casting|CastToWI_Interact (UserInterface|GetWidget (Variables|Default|GetWidget))))
  (Utilities|FlowControl|Sequence
    (:then_0
      (bind _newtrack_0 (Timeline|Timeline Play)
        (:Update
          (Class|TextBlock|SetOpacity (Variables|/Game/DEV/Taylor/Widgets/WI_Interact.WI_Interact_C|GetButtonPrompt _aswi_interact) _newtrack_0)
          (Class|Image|SetOpacity (Variables|/Game/DEV/Taylor/Widgets/WI_Interact.WI_Interact_C|GetImage_0 _aswi_interact) _newtrack_0))))))

(event Custom|HidePrompt
  (bind _newtrack_0 (Timeline|Timeline Reverse)
    (:Update
      (Class|TextBlock|SetOpacity (Variables|/Game/DEV/Taylor/Widgets/WI_Interact.WI_Interact_C|GetButtonPrompt (stale Custom|ShowPrompt _aswi_interact)) _newtrack_0)
      (Class|Image|SetOpacity (Variables|/Game/DEV/Taylor/Widgets/WI_Interact.WI_Interact_C|GetImage_0 (stale Custom|ShowPrompt _aswi_interact)) _newtrack_0))))

(event EventBeginPlay
  (bind _aswi_interact (Utilities|Casting|CastToWI_Interact (UserInterface|GetWidget (Variables|Default|GetWidget))))
  (Class|TextBlock|SetOpacity (Variables|/Game/DEV/Taylor/Widgets/WI_Interact.WI_Interact_C|GetButtonPrompt _aswi_interact) 0.0)
  (Class|Image|SetOpacity (Variables|/Game/DEV/Taylor/Widgets/WI_Interact.WI_Interact_C|GetImage_0 _aswi_interact) 0.0)
  (bind _aswi_interact_2 (Utilities|Casting|CastToWI_Interact (UserInterface|GetWidget (Variables|Default|GetWidget))))
  (Variables|/Script/UMG.TextBlock|SetText (Variables|/Game/DEV/Taylor/Widgets/WI_Interact.WI_Interact_C|GetButtonPrompt _aswi_interact_2) (Variables|Default|GetPrompt))
  (Variables|/Script/UMG.TextBlock|SetText (Variables|/Game/DEV/Taylor/Widgets/WI_Interact.WI_Interact_C|GetFunction _aswi_interact_2) (Variables|Default|GetFunc)))

(event Collision|EventActorBeginOverlap
  (params (OtherActor :type Actor%20Object%20Reference)))

(event EventTick
  (params (DeltaSeconds :type Float%20%28single-precision%29)))

(fn ConstructionScript)