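; Test NPC actor that talks to the player through a fading world-space dialogue widget and an inquire menu.
; Primary interaction shows generic or quest lines, optionally checking for and consuming a carried item, and can lock input for multi-line conversations.
; Secondary interaction opens the player's inquire box, with responses chosen by result and objective topic.
; Timelines drive fades, text length sets display time, and completed quest conversations report objective progress.
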(event Custom|ConnectionLevelChange
  (params (Connection :type Float%20%28double-precision%29))
  (bind _output_get (Variables|Default|SetConnectionLevel (+ (Variables|Default|GetConnectionLevel) Connection)))
  (Development|PrintString (Utilities|String|ToString(Float) _output_get)))

(event Custom|ShowDialogue
  (bind _questdialogue (Variables|Default|GetQuestDialogue))
  (bind _returnvalue (Utilities|Array|LastIndex _questdialogue))
  ;[0.05127 0.05127 0.05127] Regular Dialogue (Primary Interaction)
  (CallFunction|MoveDialogueBox)
  (bind _asbp_interact_prompt (Utilities|Casting|CastToBP_InteractPrompt (Variables|/Script/Engine.ChildActorComponent|GetChildActor (Variables|Default|GetBP_InteractPrompt))))
  (Variables|/Game/DEV/Taylor/BP_Actors/BP_InteractPrompt.BP_InteractPrompt_C|SetCanInteract? _asbp_interact_prompt false)
  (bind _aswi_dialogue (Utilities|Casting|CastToWI_Dialogue (UserInterface|GetWidget (Variables|Default|GetWidget))))
  (Utilities|FlowControl|Sequence
    (:then_0
      (bind _newtrack_0 (Timeline|Timeline Play)
        (:Update
          (Widget|SetRenderOpacity (Variables|/Game/DEV/Taylor/Widgets/WI_Dialogue.WI_Dialogue_C|GetVertBox_Text _aswi_dialogue) _newtrack_0)
          (CallFunction|SetOutlineOpacity (Variables|/Game/DEV/Taylor/Widgets/WI_Dialogue.WI_Dialogue_C|GetBorder_12 _aswi_dialogue) _newtrack_0)
          (Utilities|FlowControl|DoOnce false :!label _label
            (:Completed
              (if (Utilities|Array|IsEmpty (Variables|Default|GetQuestDialogue))
                (CallFunction|GenericDialogueText)
                (else
                  (bind _requirementmet (CallFunction|QuestDialogueText))
                  (if (Math|Boolean|ANDBoolean (Variables|Default|GetQuestDialogueConversation) (not (Variables|Default|GetInConversation)) _requirementmet)
                    (Input|DisableInput (Game|GetPlayerCharacter 0) (Game|GetPlayerController 0))
                    (Variables|Default|SetInConversation true)
                    (Utilities|LoopwithDelay _returnvalue _returnvalue
                      (:Loop
                        (CallFunction|ShowDialogue))
                      (:Finished
                        (Variables|Default|SetInConversation false)
                        (Input|EnableInput (Game|GetPlayerCharacter 0) (Game|GetPlayerController 0))
                        (Variables|/Game/DEV/Taylor/BP_Actors/BP_InteractPrompt.BP_InteractPrompt_C|SetCanInteract? _asbp_interact_prompt true)
                        (bind _asbp_tp_interface_example (Utilities|Casting|CastToBP_TP_InterfaceExample (Game|GetPlayerCharacter 0)))
                        (Default|ObjectiveProgress _asbp_tp_interface_example (Utilities|String|ToString(Name) (Variables|Default|GetNPCName)))))))))))
        (:Finished
          (bind _aswi_dialogue_2 (Utilities|Casting|CastToWI_Dialogue (UserInterface|GetWidget (Variables|Default|GetWidget))))
          (Utilities|FlowControl|Delay (+ (/ (Math|Conversions|ToFloat(Integer) (Utilities|String|Len (Utilities|String|ToString(Text) (Variables|/Script/UMG.MultiLineEditableTextBox|GetText (Variables|/Game/DEV/Taylor/Widgets/WI_Dialogue.WI_Dialogue_C|GetMultiLineEditableTextBox_349 _aswi_dialogue_2))))) 15.0) 1.0))
          (CallFunction|DialogueFinished)
          (Utilities|FlowControl|Delay 0.3)
          (goto _label Reset))))
    (:then_1
      (Utilities|FlowControl|DoOnce false) ; enters at Reset
    )))

(event Custom|InquireQuestFinished
  (params (SelectedIcons :type Array%20of%20Texture%202D%20Object%20References))
  (if (Utilities|Array|IsNotEmpty SelectedIcons)
    (Utilities|FlowControl|Delay 1.0)
    (Utilities|FlowControl|Delay (Variables|Default|GetInquireResponseLength))
    (bind _asbp_tp_interface_example (Utilities|Casting|CastToBP_TP_InterfaceExample (Game|GetPlayerCharacter 0)))))

(event Custom|Inquire
  (bind _returnvalue (Game|GetPlayerController 0))
  ;[0.05127 0.05127 0.05127] Inquire (Secondary Interaction)
  (CallFunction|MoveDialogueBox)
  (bind _asbp_interact_prompt (Utilities|Casting|CastToBP_InteractPrompt (Variables|/Script/Engine.ChildActorComponent|GetChildActor (Variables|Default|GetBP_InteractPrompt))))
  (Variables|/Game/DEV/Taylor/BP_Actors/BP_InteractPrompt.BP_InteractPrompt_C|SetCanInteract? _asbp_interact_prompt false)
  (Input|DisableInput (Game|GetPlayerCharacter 0) _returnvalue)
  (Variables|/Script/Engine.PlayerController|SetbShowMouseCursor _returnvalue true)
  (bind _asbp_tp_interface_example (Utilities|Casting|CastToBP_TP_InterfaceExample (Game|GetPlayerCharacter 0)))
  (bind _aswi_dialogue_box (Utilities|Casting|CastToWI_DialogueBox (UserInterface|GetWidget (Variables|/Game/DEV/Taylor/BP_CC/BP_TP_InterfaceExample.BP_TP_InterfaceExample_C|GetInquire _asbp_tp_interface_example))))
  (Default|SetParent _aswi_dialogue_box self (Variables|Default|GetLikedItems) (Variables|Default|GetInquireMin) (Variables|Default|GetInquireMax))
  (Default|Opened _aswi_dialogue_box)
  (bind _aswi_dialogue (Utilities|Casting|CastToWI_Dialogue (UserInterface|GetWidget (Variables|Default|GetWidget))))
  (bind _asbp_tp_interface_example_2 (Utilities|Casting|CastToBP_TP_InterfaceExample (Game|GetPlayerCharacter 0)))
  (bind _aswi_dialogue_box_2 (Utilities|Casting|CastToWI_DialogueBox (UserInterface|GetWidget (Variables|/Game/DEV/Taylor/BP_CC/BP_TP_InterfaceExample.BP_TP_InterfaceExample_C|GetInquire _asbp_tp_interface_example_2))))
  (bind _newtrack_0 (Timeline|Timeline_0 Play)
    (:Update
      (Widget|SetRenderOpacity (Variables|/Game/DEV/Taylor/Widgets/WI_Dialogue.WI_Dialogue_C|GetVertBox_Inquire _aswi_dialogue) _newtrack_0)
      (CallFunction|SetOutlineOpacity (Variables|/Game/DEV/Taylor/Widgets/WI_Dialogue.WI_Dialogue_C|GetBorder _aswi_dialogue) _newtrack_0))))

(event Custom|DialogueboxClosed
  ;[0.05127 0.05127 0.05127] Inquire (Secondary Interaction)
  (bind _newtrack_0 (Timeline|Timeline_0 Reverse)
    (:Update
      (Widget|SetRenderOpacity (Variables|/Game/DEV/Taylor/Widgets/WI_Dialogue.WI_Dialogue_C|GetVertBox_Inquire (stale Custom|Inquire _aswi_dialogue)) _newtrack_0)
      (CallFunction|SetOutlineOpacity (Variables|/Game/DEV/Taylor/Widgets/WI_Dialogue.WI_Dialogue_C|GetBorder (stale Custom|Inquire _aswi_dialogue)) _newtrack_0))))

(event Custom|NPCDialogueFinished
  (bind _aswi_dialogue (Utilities|Casting|CastToWI_Dialogue (UserInterface|GetWidget (Variables|Default|GetWidget))))
  (bind _newtrack_0 (Timeline|Timeline_1 ReverseFromEnd)
    (:Update
      (Widget|SetRenderOpacity (Variables|/Game/DEV/Taylor/Widgets/WI_Dialogue.WI_Dialogue_C|GetVertBox_Inquire _aswi_dialogue) _newtrack_0)
      (CallFunction|SetOutlineOpacity (Variables|/Game/DEV/Taylor/Widgets/WI_Dialogue.WI_Dialogue_C|GetBorder _aswi_dialogue) _newtrack_0))
    (:Finished
      (Utilities|FlowControl|Delay 2.3)
      (Widget|SetRenderOpacity _aswi_dialogue 1.0))))

(event Custom|DialogueFinished
  (bind _questdialogue (Variables|Default|GetQuestDialogue))
  (bind _returnvalue (Utilities|Array|LastIndex _questdialogue))
  ;[0.05127 0.05127 0.05127] Regular Dialogue (Primary Interaction)
  (Utilities|FlowControl|DoOnce false
    (:Completed
      (Utilities|FlowControl|Sequence
        (:then_0
          (bind _newtrack_0 (Timeline|Timeline Reverse)
            (:Update
              (Widget|SetRenderOpacity (Variables|/Game/DEV/Taylor/Widgets/WI_Dialogue.WI_Dialogue_C|GetVertBox_Text (stale Custom|ShowDialogue _aswi_dialogue)) _newtrack_0)
              (CallFunction|SetOutlineOpacity (Variables|/Game/DEV/Taylor/Widgets/WI_Dialogue.WI_Dialogue_C|GetBorder_12 (stale Custom|ShowDialogue _aswi_dialogue)) _newtrack_0)
              (Utilities|FlowControl|DoOnce false :!label _label
                (:Completed
                  (if (Utilities|Array|IsEmpty (Variables|Default|GetQuestDialogue))
                    (CallFunction|GenericDialogueText)
                    (else
                      (bind _requirementmet (CallFunction|QuestDialogueText))
                      (if (Math|Boolean|ANDBoolean (Variables|Default|GetQuestDialogueConversation) (not (Variables|Default|GetInConversation)) _requirementmet)
                        (Input|DisableInput (Game|GetPlayerCharacter 0) (Game|GetPlayerController 0))
                        (Variables|Default|SetInConversation true)
                        (Utilities|LoopwithDelay _returnvalue _returnvalue
                          (:Loop
                            (CallFunction|ShowDialogue))
                          (:Finished
                            (Variables|Default|SetInConversation false)
                            (Input|EnableInput (Game|GetPlayerCharacter 0) (Game|GetPlayerController 0))
                            (Variables|/Game/DEV/Taylor/BP_Actors/BP_InteractPrompt.BP_InteractPrompt_C|SetCanInteract? (stale Custom|ShowDialogue _asbp_interact_prompt) true)
                            (bind _asbp_tp_interface_example (Utilities|Casting|CastToBP_TP_InterfaceExample (Game|GetPlayerCharacter 0)))
                            (Default|ObjectiveProgress _asbp_tp_interface_example (Utilities|String|ToString(Name) (Variables|Default|GetNPCName)))))))))))
            (:Finished
              (bind _aswi_dialogue (Utilities|Casting|CastToWI_Dialogue (UserInterface|GetWidget (Variables|Default|GetWidget))))
              (Utilities|FlowControl|Delay (+ (/ (Math|Conversions|ToFloat(Integer) (Utilities|String|Len (Utilities|String|ToString(Text) (Variables|/Script/UMG.MultiLineEditableTextBox|GetText (Variables|/Game/DEV/Taylor/Widgets/WI_Dialogue.WI_Dialogue_C|GetMultiLineEditableTextBox_349 _aswi_dialogue))))) 15.0) 1.0))
              (CallFunction|DialogueFinished)
              (Utilities|FlowControl|Delay 0.3)
              (goto _label Reset))))
        (:then_1
          (if (not (Variables|Default|GetInConversation))
            (Variables|/Game/DEV/Taylor/BP_Actors/BP_InteractPrompt.BP_InteractPrompt_C|SetCanInteract? (stale Custom|ShowDialogue _asbp_interact_prompt) true)))))))

(event Custom|DialogueFinish
  ;[0.05127 0.05127 0.05127] Inquire (Secondary Interaction)
  (bind _newtrack_0 (Timeline|Timeline_0 SetNewTime)
    (:Update
      (Widget|SetRenderOpacity (Variables|/Game/DEV/Taylor/Widgets/WI_Dialogue.WI_Dialogue_C|GetVertBox_Inquire (stale Custom|Inquire _aswi_dialogue)) _newtrack_0)
      (CallFunction|SetOutlineOpacity (Variables|/Game/DEV/Taylor/Widgets/WI_Dialogue.WI_Dialogue_C|GetBorder (stale Custom|Inquire _aswi_dialogue)) _newtrack_0))))

(event Custom|InquireResponse
  (params (GoodResult? :type Boolean) (DialogueBox :type WI%20Dialogue%20Box%20Object%20Reference) (NewParam :type Array%20of%20Texture%202D%20Object%20References))
  (bind _inquirequestdialogue (Variables|Default|GetInquireQuestDialogue))
  (bind _returnvalue (Utilities|Array|LastIndex _inquirequestdialogue))
  ;[0.05127 0.05127 0.05127] Inquire Response
  (bind _aswi_dialogue (Utilities|Casting|CastToWI_Dialogue (UserInterface|GetWidget (Variables|Default|GetWidget))))
  (Utilities|FlowControl|Sequence
    (:then_0
      (bind _newtrack_0 (Timeline|Timeline_2 Play)
        (:Update
          (Widget|SetRenderOpacity (Variables|/Game/DEV/Taylor/Widgets/WI_Dialogue.WI_Dialogue_C|GetVertBox_Text _aswi_dialogue) _newtrack_0)
          (CallFunction|SetOutlineOpacity (Variables|/Game/DEV/Taylor/Widgets/WI_Dialogue.WI_Dialogue_C|GetBorder_12 _aswi_dialogue) _newtrack_0)
          (Utilities|FlowControl|DoOnce false :!label _label
            (:Completed
              (bind _objective (Utilities|GetObjective)
                (:output
                  (if (Utilities|Enum|Equal(Enum) (.ObjectiveID (Utilities|Struct|BreakS_ObjectiveDetails _objective)) (Utilities|String|ToString(Name) (Variables|Default|GetNPCName)))
                    (Utilities|FlowControl|DoOnce false :!label _label_2
                      (:Completed
                        (if (or (Utilities|Array|IsEmpty (Variables|Default|GetInquireQuestDialogue)) (not (Utilities|Array|ContainsItem (Variables|/Game/DEV/Taylor/Widgets/WI_DialogueBox.WI_DialogueBox_C|GetSelectedIcons DialogueBox) (.InquireTopics (Utilities|Struct|BreakS_ObjectiveDetails _objective)))))
                          (CallFunction|InquireResponseText GoodResult?)
                          (else
                            (CallFunction|QuestInquireDialogueText)
                            (if (not (Variables|Default|GetInConversation))
                              (Input|DisableInput (Game|GetPlayerCharacter 0) (Game|GetPlayerController 0))
                              (Variables|Default|SetInConversation true)
                              (Utilities|LoopwithDelay _returnvalue _returnvalue
                                (:Loop
                                  (CallFunction|InquireResponse GoodResult? DialogueBox NewParam))
                                (:Finished
                                  (Variables|Default|SetInConversation false)
                                  (Input|EnableInput (Game|GetPlayerCharacter 0) (Game|GetPlayerController 0))
                                  (bind _asbp_tp_interface_example (Utilities|Casting|CastToBP_TP_InterfaceExample (Game|GetPlayerCharacter 0)))
                                  (Default|InquireFinished DialogueBox)
                                  (Default|ObjectiveProgress _asbp_tp_interface_example (Utilities|String|ToString(Name) (Variables|Default|GetNPCName)) NewParam))))))))))
                (:Completed
                  (Utilities|FlowControl|Sequence
                    (:then_0
                      (goto _label_2))
                    (:then_1
                      (goto _label_2 Reset))))))))
        (:Finished
          (bind _aswi_dialogue_2 (Utilities|Casting|CastToWI_Dialogue (UserInterface|GetWidget (Variables|Default|GetWidget))))
          (Variables|Default|SetInquireResponseLength (+ (/ (Math|Conversions|ToFloat(Integer) (Utilities|String|Len (Utilities|String|ToString(Text) (Variables|/Script/UMG.MultiLineEditableTextBox|GetText (Variables|/Game/DEV/Taylor/Widgets/WI_Dialogue.WI_Dialogue_C|GetMultiLineEditableTextBox_349 _aswi_dialogue_2))))) 15.0) 1.0))
          (Utilities|FlowControl|Delay (+ (/ (Math|Conversions|ToFloat(Integer) (Utilities|String|Len (Utilities|String|ToString(Text) (Variables|/Script/UMG.MultiLineEditableTextBox|GetText (Variables|/Game/DEV/Taylor/Widgets/WI_Dialogue.WI_Dialogue_C|GetMultiLineEditableTextBox_349 _aswi_dialogue_2))))) 15.0) 1.0))
          (CallFunction|InquireResponseFinished)
          (Utilities|FlowControl|Delay 0.3)
          (goto _label Reset))))
    (:then_1
      (Utilities|FlowControl|DoOnce false) ; enters at Reset
    )))

(event Custom|InquireResponseFinished
  (bind _inquirequestdialogue (Variables|Default|GetInquireQuestDialogue))
  (bind _returnvalue (Utilities|Array|LastIndex _inquirequestdialogue))
  ;[0.05127 0.05127 0.05127] Inquire Response
  (Utilities|FlowControl|DoOnce false
    (:Completed
      (Utilities|FlowControl|Sequence
        (:then_0
          (bind _newtrack_0 (Timeline|Timeline_2 Reverse)
            (:Update
              (Widget|SetRenderOpacity (Variables|/Game/DEV/Taylor/Widgets/WI_Dialogue.WI_Dialogue_C|GetVertBox_Text (stale Custom|InquireResponse _aswi_dialogue)) _newtrack_0)
              (CallFunction|SetOutlineOpacity (Variables|/Game/DEV/Taylor/Widgets/WI_Dialogue.WI_Dialogue_C|GetBorder_12 (stale Custom|InquireResponse _aswi_dialogue)) _newtrack_0)
              (Utilities|FlowControl|DoOnce false :!label _label
                (:Completed
                  (bind _objective (Utilities|GetObjective)
                    (:output
                      (if (Utilities|Enum|Equal(Enum) (.ObjectiveID (Utilities|Struct|BreakS_ObjectiveDetails _objective)) (Utilities|String|ToString(Name) (Variables|Default|GetNPCName)))
                        (Utilities|FlowControl|DoOnce false :!label _label_2
                          (:Completed
                            (if (or (Utilities|Array|IsEmpty (Variables|Default|GetInquireQuestDialogue)) (not (Utilities|Array|ContainsItem (Variables|/Game/DEV/Taylor/Widgets/WI_DialogueBox.WI_DialogueBox_C|GetSelectedIcons (stale Custom|InquireResponse DialogueBox)) (.InquireTopics (Utilities|Struct|BreakS_ObjectiveDetails _objective)))))
                              (CallFunction|InquireResponseText (stale Custom|InquireResponse GoodResult?))
                              (else
                                (CallFunction|QuestInquireDialogueText)
                                (if (not (Variables|Default|GetInConversation))
                                  (Input|DisableInput (Game|GetPlayerCharacter 0) (Game|GetPlayerController 0))
                                  (Variables|Default|SetInConversation true)
                                  (Utilities|LoopwithDelay _returnvalue _returnvalue
                                    (:Loop
                                      (CallFunction|InquireResponse (stale Custom|InquireResponse GoodResult?) (stale Custom|InquireResponse DialogueBox) (stale Custom|InquireResponse NewParam)))
                                    (:Finished
                                      (Variables|Default|SetInConversation false)
                                      (Input|EnableInput (Game|GetPlayerCharacter 0) (Game|GetPlayerController 0))
                                      (bind _asbp_tp_interface_example (Utilities|Casting|CastToBP_TP_InterfaceExample (Game|GetPlayerCharacter 0)))
                                      (Default|InquireFinished (stale Custom|InquireResponse DialogueBox))
                                      (Default|ObjectiveProgress _asbp_tp_interface_example (Utilities|String|ToString(Name) (Variables|Default|GetNPCName)) (stale Custom|InquireResponse NewParam)))))))))))
                    (:Completed
                      (Utilities|FlowControl|Sequence
                        (:then_0
                          (goto _label_2))
                        (:then_1
                          (goto _label_2 Reset))))))))
            (:Finished
              (bind _aswi_dialogue (Utilities|Casting|CastToWI_Dialogue (UserInterface|GetWidget (Variables|Default|GetWidget))))
              (Variables|Default|SetInquireResponseLength (+ (/ (Math|Conversions|ToFloat(Integer) (Utilities|String|Len (Utilities|String|ToString(Text) (Variables|/Script/UMG.MultiLineEditableTextBox|GetText (Variables|/Game/DEV/Taylor/Widgets/WI_Dialogue.WI_Dialogue_C|GetMultiLineEditableTextBox_349 _aswi_dialogue))))) 15.0) 1.0))
              (Utilities|FlowControl|Delay (+ (/ (Math|Conversions|ToFloat(Integer) (Utilities|String|Len (Utilities|String|ToString(Text) (Variables|/Script/UMG.MultiLineEditableTextBox|GetText (Variables|/Game/DEV/Taylor/Widgets/WI_Dialogue.WI_Dialogue_C|GetMultiLineEditableTextBox_349 _aswi_dialogue))))) 15.0) 1.0))
              (CallFunction|InquireResponseFinished)
              (Utilities|FlowControl|Delay 0.3)
              (goto _label Reset))))
        (:then_1
          (if (not (Variables|Default|GetInConversation))
            (Default|InquireFinished (stale Custom|InquireResponse DialogueBox))))))))

(event Custom|MoveTo
  (params (Destination :type Vector))
  (AI|AIMoveTo self Destination 0 5.0 false
    (:OnSuccess
      _)
    (:OnFail
      _))
  (Transformation|SetActorRotation "0, 0, 0"))

(event EventBeginPlay)

(event Collision|EventActorBeginOverlap
  (params (OtherActor :type Actor%20Object%20Reference)))

(event EventTick
  (params (DeltaSeconds :type Float%20%28single-precision%29)))

(event EventGeneralInteract
  ;[0.05127 0.05127 0.05127] Primary Interaction
  (bind _asbp_interact_prompt (Utilities|Casting|CastToBP_InteractPrompt (Variables|/Script/Engine.ChildActorComponent|GetChildActor (Variables|Default|GetBP_InteractPrompt))))
  (if (Variables|/Game/DEV/Taylor/BP_Actors/BP_InteractPrompt.BP_InteractPrompt_C|GetCanInteract? _asbp_interact_prompt)
    (CallFunction|ShowDialogue)))

(event EventShowPrompt
  ;[0.05127 0.05127 0.05127] ButtonPrompt
  (bind _asbp_interact_prompt (Utilities|Casting|CastToBP_InteractPrompt (Variables|/Script/Engine.ChildActorComponent|GetChildActor (Variables|Default|GetBP_InteractPrompt))))
  (Default|ShowPrompt _asbp_interact_prompt))

(event EventInteractE
  ;[0.05127 0.05127 0.05127] Secondary Interaction
  (bind _asbp_interact_prompt (Utilities|Casting|CastToBP_InteractPrompt (Variables|/Script/Engine.ChildActorComponent|GetChildActor (Variables|Default|GetBP_InteractPrompt))))
  (if (Variables|/Game/DEV/Taylor/BP_Actors/BP_InteractPrompt.BP_InteractPrompt_C|GetCanInteract? _asbp_interact_prompt)
    (CallFunction|Inquire)))

(fn ConstructionScript)

(fn GenericDialogueText
  (bind _aswi_dialogue (Utilities|Casting|CastToWI_Dialogue (UserInterface|GetWidget (Variables|Default|GetWidget))))
  (Variables|/Script/UMG.MultiLineEditableTextBox|SetText (Variables|/Game/DEV/Taylor/Widgets/WI_Dialogue.WI_Dialogue_C|GetMultiLineEditableTextBox_349 _aswi_dialogue) (Utilities|Text|ToText(String) (Utilities|Array|Get(acopy) (Variables|Default|GetDialogue) (Variables|Default|GetArrayIndex))))
  (bind _output_get (Variables|Default|SetArrayIndex (+ (Variables|Default|GetArrayIndex) 1)))
  (if (> _output_get (Utilities|Array|LastIndex (Variables|Default|GetDialogue)))
    (Variables|Default|SetArrayIndex 0)))

(fn MoveDialogueBox
  (bind _widget (Variables|Default|GetWidget))
  (bind _widget_2 (Variables|Default|GetWidget))
  (bind _returnvalue (UserInterface|GetWidget _widget_2))
  (if (Variables|Default|GetAutomateDialogueMovement?)
    (if (>= (.y (Transformation|GetWorldLocation (Variables|/Script/Engine.Character|GetCapsuleComponent (Game|GetPlayerCharacter 0)))) (.y (Transformation|GetWorldLocation (Variables|Collision|GetCapsuleComponent))))
      (Transformation|SetRelativeLocation _widget (Math|Vector|MakeVector 0.0 -175.0 135.0) false false)
      (bind _aswi_dialogue (Utilities|Casting|CastToWI_Dialogue _returnvalue))
      (Variables|/Script/UMG.Widget|SetRenderTransform (Variables|/Game/DEV/Taylor/Widgets/WI_Dialogue.WI_Dialogue_C|GetCanvasPanel_344 _aswi_dialogue) (Utilities|Struct|MakeWidgetTransform "(X=0.000000,Y=0.000000)" "(X=-1.000000,Y=1.000000)" "(X=0.000000,Y=0.000000)" 1.8e+02))
      (Variables|/Script/UMG.Widget|SetRenderTransform (Variables|/Game/DEV/Taylor/Widgets/WI_Dialogue.WI_Dialogue_C|GetCanvasPanel _aswi_dialogue) (Utilities|Struct|MakeWidgetTransform "(X=0.000000,Y=0.000000)" "(X=-1.000000,Y=1.000000)" "(X=0.000000,Y=0.000000)" 1.8e+02))
      (else
        (Transformation|SetRelativeLocation _widget (Math|Vector|MakeVector 0.0 175.0 135.0) false false)
        (bind _aswi_dialogue_2 (Utilities|Casting|CastToWI_Dialogue _returnvalue))
        (Variables|/Script/UMG.Widget|SetRenderTransform (Variables|/Game/DEV/Taylor/Widgets/WI_Dialogue.WI_Dialogue_C|GetCanvasPanel_344 _aswi_dialogue_2) (Utilities|Struct|MakeWidgetTransform "(X=0.000000,Y=0.000000)" "(X=1.000000,Y=1.000000)" "(X=0.000000,Y=0.000000)" 1.8e+02))
        (Variables|/Script/UMG.Widget|SetRenderTransform (Variables|/Game/DEV/Taylor/Widgets/WI_Dialogue.WI_Dialogue_C|GetCanvasPanel _aswi_dialogue_2) (Utilities|Struct|MakeWidgetTransform "(X=0.000000,Y=0.000000)" "(X=1.000000,Y=1.000000)" "(X=0.000000,Y=0.000000)" 1.8e+02))))))

(fn InquireResponseText
  (params (Result :type Boolean))
  (if Result
    (bind _aswi_dialogue (Utilities|Casting|CastToWI_Dialogue (UserInterface|GetWidget (Variables|Default|GetWidget))))
    (Variables|/Script/UMG.MultiLineEditableTextBox|SetText (Variables|/Game/DEV/Taylor/Widgets/WI_Dialogue.WI_Dialogue_C|GetMultiLineEditableTextBox_349 _aswi_dialogue) (Utilities|Text|ToText(String) (Utilities|Array|Get(acopy) (Variables|Default|GetInquireDialogue) (Variables|Default|GetInquireResponseArrayIndex))))
    (Widget|Panel|ClearChildren (Variables|/Game/DEV/Taylor/Widgets/WI_Dialogue.WI_Dialogue_C|GetWrapBox_77 _aswi_dialogue))
    (bind _output_get (Variables|Default|SetInquireResponseArrayIndex (+ (Variables|Default|GetInquireResponseArrayIndex) 1)))
    (if (> _output_get (Utilities|Array|LastIndex (Variables|Default|GetInquireDialogue)))
      (Variables|Default|SetInquireResponseArrayIndex (Utilities|Array|LastIndex (Variables|Default|GetInquireDialogue))))
    (else
      (bind _aswi_dialogue_2 (Utilities|Casting|CastToWI_Dialogue (UserInterface|GetWidget (Variables|Default|GetWidget))))
      (Variables|/Script/UMG.MultiLineEditableTextBox|SetText (Variables|/Game/DEV/Taylor/Widgets/WI_Dialogue.WI_Dialogue_C|GetMultiLineEditableTextBox_349 _aswi_dialogue_2) (Utilities|Text|ToText(String) (Utilities|Array|Get(acopy) (Variables|Default|GetInquireBadConversation) (Variables|Default|GetNotInterestedArrayIndex))))
      (Widget|Panel|ClearChildren (Variables|/Game/DEV/Taylor/Widgets/WI_Dialogue.WI_Dialogue_C|GetWrapBox_77 _aswi_dialogue_2))
      (bind _output_get_2 (Variables|Default|SetNotInterestedArrayIndex (+ (Variables|Default|GetNotInterestedArrayIndex) 1)))
      (if (> _output_get_2 (Utilities|Array|LastIndex (Variables|Default|GetInquireBadConversation)))
        (Variables|Default|SetNotInterestedArrayIndex 0)))))

(fn SetOutlineOpacity
  (params (Outline :type Border%20Object%20Reference) (Opacity :type Float%20%28double-precision%29))
  (bind _background (Variables|/Script/UMG.Border|GetBackground Outline))
  (Class|Border|SetBrush Outline (Utilities|Struct|MakeSlateBrush (.drawas _background) (.tiling _background) (.mirroring _background) (.imagesize _background) (.margin _background) (.tintcolor _background) (Utilities|Struct|MakeSlateBrushOutlineSettings (.cornerradii (.outlinesettings _background)) (Utilities|Struct|MakeSlateColor (Utilities|Struct|MakeLinearColor (.r (.specifiedcolor (.color (.outlinesettings _background)))) (.g (.specifiedcolor (.color (.outlinesettings _background)))) (.b (.specifiedcolor (.color (.outlinesettings _background)))) Opacity) (.coloruserule (.color (.outlinesettings _background)))) (.width (.outlinesettings _background)) (.roundingtype (.outlinesettings _background)) (.busebrushtransparency (.outlinesettings _background))) (.resourceobject _background))))

(fn QuestDialogueText
  (if (Utilities|IsValidClass (Variables|Default|GetRequireditem))
    (bind _asbp_tp_interface_example (Utilities|Casting|CastToBP_TP_InterfaceExample (Game|GetPlayerCharacter 0)))
    (Utilities|IsValid (Variables|/Game/DEV/Taylor/BP_CC/BP_TP_InterfaceExample.BP_TP_InterfaceExample_C|GetBag _asbp_tp_interface_example)
      (:Is%20Valid
        (if (== (Utilities|GetClass (Variables|/Game/DEV/Taylor/BP_CC/BP_TP_InterfaceExample.BP_TP_InterfaceExample_C|GetBag _asbp_tp_interface_example)) (Variables|Default|GetRequireditem))
          _
          (else
            (bind _aswi_dialogue (Utilities|Casting|CastToWI_Dialogue (UserInterface|GetWidget (Variables|Default|GetWidget)) :!label _label))
            (Variables|/Script/UMG.MultiLineEditableTextBox|SetText (Variables|/Game/DEV/Taylor/Widgets/WI_Dialogue.WI_Dialogue_C|GetMultiLineEditableTextBox_349 _aswi_dialogue) (Utilities|Text|ToText(String) (Variables|Default|GetRequiredDialogueNotMet)))
            (return false))))
      (:Is%20Not%20Valid
        (goto _label))))
  (bind _aswi_dialogue_2 (Utilities|Casting|CastToWI_Dialogue (UserInterface|GetWidget (Variables|Default|GetWidget))))
  (Variables|/Script/UMG.MultiLineEditableTextBox|SetText (Variables|/Game/DEV/Taylor/Widgets/WI_Dialogue.WI_Dialogue_C|GetMultiLineEditableTextBox_349 _aswi_dialogue_2) (Utilities|Text|ToText(String) (Utilities|Array|Get(acopy) (Variables|Default|GetQuestDialogue) (Variables|Default|GetQuestDialogueArrayIndex))))
  (bind _output_get (Variables|Default|SetQuestDialogueArrayIndex (+ (Variables|Default|GetQuestDialogueArrayIndex) 1)))
  (if (> _output_get (Utilities|Array|LastIndex (Variables|Default|GetQuestDialogue)))
    (Variables|Default|SetQuestDialogueArrayIndex 0)
    (Utilities|IsValid (Variables|/Game/DEV/Taylor/BP_CC/BP_TP_InterfaceExample.BP_TP_InterfaceExample_C|GetBag _asbp_tp_interface_example)
      (:Is%20Valid
        (Actor|DestroyActor (Variables|/Game/DEV/Taylor/BP_CC/BP_TP_InterfaceExample.BP_TP_InterfaceExample_C|GetBag _asbp_tp_interface_example))
        (Variables|/Game/DEV/Taylor/BP_CC/BP_TP_InterfaceExample.BP_TP_InterfaceExample_C|SetCarryingObject _asbp_tp_interface_example false))
      (:Is%20Not%20Valid
        _))
    (return true)
    (else
      (return true))))

(fn QuestInquireDialogueText
  (bind _aswi_dialogue (Utilities|Casting|CastToWI_Dialogue (UserInterface|GetWidget (Variables|Default|GetWidget))))
  (Variables|/Script/UMG.MultiLineEditableTextBox|SetText (Variables|/Game/DEV/Taylor/Widgets/WI_Dialogue.WI_Dialogue_C|GetMultiLineEditableTextBox_349 _aswi_dialogue) (Utilities|Text|ToText(String) (Utilities|Array|Get(acopy) (Variables|Default|GetInquireQuestDialogue) (Variables|Default|GetQuestDialogueArrayIndex))))
  (bind _output_get (Variables|Default|SetQuestDialogueArrayIndex (+ (Variables|Default|GetQuestDialogueArrayIndex) 1)))
  (if (> _output_get (Utilities|Array|LastIndex (Variables|Default|GetInquireQuestDialogue)))
    (Variables|Default|SetQuestDialogueArrayIndex 0)))

(fn GiveQuest
  (Default|GiveQuest (Variables|Default|GetQuestGiverComponent))
  (return (Utilities|String|ToString(Name) (Variables|Default|GetNPCName))))