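; Pickup actor that animates its mesh's height and yaw with a Timeline from BeginPlay.
; On GeneralInteract it casts the player character to BP_TP_InterfaceExample, passes it the item icon and name through PickUp, then destroys itself.
; ShowPrompt forwards to a BP_InteractPrompt child actor.
; The construction script applies the configured mesh and per-slot materials, so each instance can look different.
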(event EventBeginPlay
  (bind (_direction _newtrack_0 _newtrack_1) (Timeline|Timeline Play)
    (:Update
      (Transformation|SetRelativeLocationAndRotation (Variables|Default|GetCube) (Math|Vector|MakeVector 0.0 0.0 _newtrack_1) (Math|Rotator|MakeRotator 0.0 0.0 _newtrack_0) false false))))

(event Collision|EventActorBeginOverlap
  (params (OtherActor :type Actor%20Object%20Reference)))

(event EventTick
  (params (DeltaSeconds :type Float%20%28single-precision%29)))

(event EventGeneralInteract
  (bind _asbp_tp_interface_example (Utilities|Casting|CastToBP_TP_InterfaceExample (Game|GetPlayerCharacter 0)))
  (Default|PickUp _asbp_tp_interface_example (Variables|Default|GetItem) (Variables|Default|GetObjectName))
  (Actor|DestroyActor))

(event EventShowPrompt
  (bind _asbp_interact_prompt (Utilities|Casting|CastToBP_InteractPrompt (Variables|/Script/Engine.ChildActorComponent|GetChildActor (Variables|Default|GetBP_InteractPrompt))))
  (Default|ShowPrompt _asbp_interact_prompt))

(fn ConstructionScript
  (if (Utilities|IsValid (Variables|Default|GetMesh))
    (Components|StaticMesh|SetStaticMesh (Variables|Default|GetCube) (Variables|Default|GetMesh))
    (for (_ _array_index) (Rendering|Material|GetMaterials (Variables|Default|GetCube))
      (Rendering|Material|SetMaterial (Variables|Default|GetCube) _array_index (Utilities|Array|Get(acopy) (Variables|Default|GetMaterial) _array_index)))))