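; BP_Rubbish is an interactable rubbish object that gives the player a bin bag to carry.
; When the player's hands are free, it shows a child-actor prompt, and interacting spawns a BP_BinBag_Pickup, then hides the rubbish and changes its collision.
; IsActive reapplies that collected state.
; Shortly after BeginPlay, a custom loop scans Quests actors' current objectives, destroying the rubbish on any non-bin objective, with debug prints.
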(event EventBeginPlay
  (Utilities|FlowControl|Delay 0.3)
  (bind _outactors (Actor|GetAllActorsOfClass "/Game/DEV/Taylor/Quests/Quests.Quests_C"))
  (Variables|Default|SetLoops 0)
  (Utilities|Loop (Utilities|Array|Length _outactors) :!label _label
    (:NewParam2
      (for _array_element (.objectives (Variables|/Game/DEV/Taylor/Quests/Quests.Quests_C|GetCurrentStageDetails (Utilities|Array|Get(acopy) _outactors (Variables|Default|GetLoops))))
        (if (Utilities|Enum|Equal(Enum) (.Type (Utilities|Struct|BreakS_ObjectiveDetails _array_element)) "NewEnumerator5")
          (Development|PrintString "BinQuest")
          (else
            (Development|PrintString "NotBinQuest")
            (Actor|DestroyActor))))
      (Math|Integer|IncrementInt (Variables|Default|GetLoops)
        (:%20%20
          (goto _label))))))

(event EventGeneralInteract
  (bind _asbp_tp_interface_example (Utilities|Casting|CastToBP_TP_InterfaceExample (Game|GetPlayerCharacter 0)))
  (if (not (Variables|/Game/DEV/Taylor/BP_CC/BP_TP_InterfaceExample.BP_TP_InterfaceExample_C|GetCarryingObject _asbp_tp_interface_example))
    (bind _returnvalue (Game|SpawnActorfromClass "/Game/DEV/Taylor/BP_Actors/BinObjects/BP_BinBag_Pickup.BP_BinBag_Pickup_C" (Math|Transform|MakeTransform "0, 0, 0" "0, 0, 0" "1.000000,1.000000,1.000000") "Undefined" "MultiplyWithRoot" 0 0))
    (Default|BinBagPickup _asbp_tp_interface_example _returnvalue)
    (Variables|Default|SetCollected? true)
    (Rendering|SetVisibility (Variables|Default|GetDefaultSceneRoot) false true)
    (Collision|SetCollisionObjectType (Variables|Default|GetSphere) "ECC_WorldDynamic")))

(event EventShowPrompt
  (bind _asbp_tp_interface_example (Utilities|Casting|CastToBP_TP_InterfaceExample (Game|GetPlayerCharacter 0)))
  (if (not (Variables|/Game/DEV/Taylor/BP_CC/BP_TP_InterfaceExample.BP_TP_InterfaceExample_C|GetCarryingObject _asbp_tp_interface_example))
    (bind _asbp_interact_prompt (Utilities|Casting|CastToBP_InteractPrompt (Variables|/Script/Engine.ChildActorComponent|GetChildActor (Variables|Default|GetBP_InteractPrompt))))
    (Default|ShowPrompt _asbp_interact_prompt)))

(fn ConstructionScript)

(fn IsActive
  (params (Collected :type Boolean))
  (bind _output_get (Variables|Default|SetCollected? Collected))
  (if _output_get
    (Rendering|SetVisibility (Variables|Default|GetDefaultSceneRoot) false true)
    (Collision|SetCollisionObjectType (Variables|Default|GetSphere) "ECC_WorldDynamic")))