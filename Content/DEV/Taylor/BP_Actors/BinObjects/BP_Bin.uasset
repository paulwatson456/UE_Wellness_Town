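; BP_Bin is a quest bin that destroys BP_BinBag actors overlapping its trigger sphere and counts them toward an objective.
; On BeginPlay, after a short delay, it scans the player's QuestComponent for objectives matching BinName to load required quantity and progress.
; Binning clears the player's carry state for attached bags, then reports progress through ObjectiveProgress.
; A hidden Sphere appears when the requirement is met or a scanned objective doesn't match.
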(event OnComponentBeginOverlap(Sphere1)
  (params (OverlappedComponent :type Primitive%20Component%20Object%20Reference) (OtherActor :type Actor%20Object%20Reference) (OtherComp :type Primitive%20Component%20Object%20Reference) (OtherBodyIndex :type Integer) (bFromSweep :type Boolean) (SweepResult :type Hit%20Result%20Structure%20%28by%20ref%29))
  (bind _asbp_bin_bag (Utilities|Casting|CastToBP_BinBag OtherActor))
  (if (>= (Variables|Default|GetObjectsBinned) (Variables|Default|GetRequirement))
    (Development|PrintString "Finished")
    (else
      (Utilities|IsValid (Transformation|GetAttachParent (Variables|/Game/DEV/Taylor/BP_Actors/BinObjects/BP_BinBag.BP_BinBag_C|GetCube _asbp_bin_bag))
        (:Is%20Valid
          (bind _asbp_tp_interface_example (Utilities|Casting|CastToBP_TP_InterfaceExample (Game|GetPlayerCharacter 0)))
          (Variables|/Game/DEV/Taylor/BP_CC/BP_TP_InterfaceExample.BP_TP_InterfaceExample_C|SetCarryingObject _asbp_tp_interface_example false)
          (Variables|/Game/DEV/Taylor/BP_CC/BP_TP_InterfaceExample.BP_TP_InterfaceExample_C|SetBag _asbp_tp_interface_example 0)
          (Actor|DestroyActor _asbp_bin_bag)
          (Development|PrintString "Carrying")
          (Math|Integer|IncrementInt (Variables|Default|GetObjectsBinned)
            (:%20%20
              (CallFunction|Finished))))
        (:Is%20Not%20Valid
          (Actor|DestroyActor _asbp_bin_bag)
          (Development|PrintString "Not carrying")
          (Math|Integer|IncrementInt (Variables|Default|GetObjectsBinned)
            (:%20%20
              (CallFunction|Finished))))))))

(event EventBeginPlay
  (bind _binname (Variables|Default|GetBinName))
  (Utilities|FlowControl|Delay 0.7)
  (bind _asbp_tp_interface_example (Utilities|Casting|CastToBP_TP_InterfaceExample (Game|GetPlayerCharacter 0)))
  (Variables|Default|SetLoops 0)
  (Utilities|Loop (Utilities|Array|Length (Variables|/Game/DEV/Taylor/Quests/QuestComponent.QuestComponent_C|GetCurrentQuests (Variables|/Game/DEV/Taylor/BP_CC/BP_TP_InterfaceExample.BP_TP_InterfaceExample_C|GetQuestComponent _asbp_tp_interface_example))) :!label _label
    (:NewParam2
      (for _array_element (.Objectives (Utilities|Struct|BreakS_StageDetails (Variables|/Game/DEV/Taylor/Quests/Quests.Quests_C|GetCurrentStageDetails (Utilities|Array|Get(acopy) (Variables|/Game/DEV/Taylor/Quests/QuestComponent.QuestComponent_C|GetCurrentQuests (Variables|/Game/DEV/Taylor/BP_CC/BP_TP_InterfaceExample.BP_TP_InterfaceExample_C|GetQuestComponent _asbp_tp_interface_example)) (Variables|Default|GetLoops)))))
        (if (and (Utilities|Enum|Equal(Enum) (.Type (Utilities|Struct|BreakS_ObjectiveDetails _array_element)) "NewEnumerator5") (Utilities|Enum|Equal(Enum) (.ObjectiveID (Utilities|Struct|BreakS_ObjectiveDetails _array_element)) _binname))
          (bind _output_get (Variables|Default|SetRequirement (.Quantity (Utilities|Struct|BreakS_ObjectiveDetails _array_element))))
          (bind _output_get_2 (Variables|Default|SetObjectsBinned (.Value (Utilities|Map|Find (Variables|/Game/DEV/Taylor/Quests/Quests.Quests_C|GetCurrentOpbectiveProgress (Utilities|Array|Get(acopy) (Variables|/Game/DEV/Taylor/Quests/QuestComponent.QuestComponent_C|GetCurrentQuests (Variables|/Game/DEV/Taylor/BP_CC/BP_TP_InterfaceExample.BP_TP_InterfaceExample_C|GetQuestComponent _asbp_tp_interface_example)) (Variables|Default|GetLoops))) _binname))))
          (Development|PrintString (Utilities|String|Append (Utilities|String|ToString(Integer) _output_get_2) " / " (Utilities|String|ToString(Integer) _output_get)))
          (else
            (Development|SetHiddeninGame (Variables|Default|GetSphere) false true))))
      (Math|Integer|IncrementInt (Variables|Default|GetLoops)
        (:%20%20
          (goto _label))))))

(event Collision|EventActorBeginOverlap
  (params (OtherActor :type Actor%20Object%20Reference)))

(event EventTick
  (params (DeltaSeconds :type Float%20%28single-precision%29)))

(fn ConstructionScript
  (Development|SetHiddeninGame (Variables|Default|GetSphere) true true))

(fn Finished
  (bind _asbp_tp_interface_example (Utilities|Casting|CastToBP_TP_InterfaceExample (Game|GetPlayerCharacter 0)))
  (Default|ObjectiveProgress _asbp_tp_interface_example (Variables|Default|GetBinName))
  (if (>= (Variables|Default|GetObjectsBinned) (Variables|Default|GetRequirement))
    (Development|SetHiddeninGame (Variables|Default|GetSphere) false true)))