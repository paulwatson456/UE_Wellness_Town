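; BP_BinBag is a physics bin bag that the player picks up.
; On interact it calls BinBagPickup on the player character if their hands are free, and it shows its child-actor interact prompt under the same condition.
; Hard hits play a bounce sound with volume scaled by the cube's velocity, throttled by a DoOnce that resets after a short delay.
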(event OnComponentHit(Cube)
  (params (HitComponent :type Primitive%20Component%20Object%20Reference) (OtherActor :type Actor%20Object%20Reference) (OtherComp :type Primitive%20Component%20Object%20Reference) (NormalImpulse :type Vector :default "0, 0, 0") (Hit :type Hit%20Result%20Structure%20%28by%20ref%29))
  (bind _cube (Variables|Default|GetCube))
  (bind _returnvalue (Transformation|GetComponentVelocity _cube))
  (bind _returnvalue_2 (Math|Vector|VectorLength _returnvalue))
  (if (> _returnvalue_2 2e+02)
    (Utilities|FlowControl|DoOnce false :!label _label
      (:Completed
        (Audio|PlaySoundatLocation "/Game/DEV/Taylor/Sound/BinBagBounce.BinBagBounce" (Transformation|GetWorldLocation _cube) "0, 0, 0" (/ _returnvalue_2 1.5e+03) 1.0 0.0 0 0 0 0)
        (Utilities|FlowControl|Delay 0.1)
        (goto _label Reset)))))

(event EventGeneralInteract
  (bind _asbp_tp_interface_example (Utilities|Casting|CastToBP_TP_InterfaceExample (Game|GetPlayerCharacter 0)))
  (if (not (Variables|/Game/DEV/Taylor/BP_CC/BP_TP_InterfaceExample.BP_TP_InterfaceExample_C|GetCarryingObject _asbp_tp_interface_example))
    (Default|BinBagPickup _asbp_tp_interface_example self)))

(event EventShowPrompt
  (bind _asbp_tp_interface_example (Utilities|Casting|CastToBP_TP_InterfaceExample (Game|GetPlayerCharacter 0)))
  (if (not (Variables|/Game/DEV/Taylor/BP_CC/BP_TP_InterfaceExample.BP_TP_InterfaceExample_C|GetCarryingObject _asbp_tp_interface_example))
    (bind _asbp_interact_prompt (Utilities|Casting|CastToBP_InteractPrompt (Variables|/Script/Engine.ChildActorComponent|GetChildActor (Variables|Default|GetBP_InteractPrompt))))
    (Default|ShowPrompt _asbp_interact_prompt)))

(fn ConstructionScript)