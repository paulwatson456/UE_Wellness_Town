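; Level-transition door that sends the player to another level and places them at the matching door on arrival.
; Overlap of the box by the BP_TP_InterfaceExample character fades the camera, waits, stores DoorName in the GI_SpawnPoints game instance, then opens LevelName.
; On BeginPlay, a door whose DoorName matches that stored spawn teleports the player to its Arrow.
; An older DoorPosition save-game version remains as unconnected nodes.
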(event OnComponentBeginOverlap(Box)
  (params (OverlappedComponent :type Primitive%20Component%20Object%20Reference) (OtherActor :type Actor%20Object%20Reference) (OtherComp :type Primitive%20Component%20Object%20Reference) (OtherBodyIndex :type Integer) (bFromSweep :type Boolean) (SweepResult :type Hit%20Result%20Structure%20%28by%20ref%29))
  (Utilities|Casting|CastToBP_TP_InterfaceExample OtherActor)
  (CallFunction|SetSpawnPos))

(event Custom|SetSpawnPos
  (CallFunction|OverlayFadein)
  (Utilities|FlowControl|Delay 0.75)
  (bind _asgi_spawn_points (Utilities|Casting|CastToGI_SpawnPoints (Game|GetGameInstance)))
  (Variables|/Game/DEV/Taylor/GameInstance/GI_SpawnPoints.GI_SpawnPoints_C|SetSpawn _asgi_spawn_points (Variables|Default|GetDoorName))
  (Game|OpenLevel(byName) (Variables|Default|GetLevelName)))

(event EventBeginPlay
  (bind _asgi_spawn_points (Utilities|Casting|CastToGI_SpawnPoints (Game|GetGameInstance)))
  (if (Utilities|Enum|Equal(Enum) (Variables|Default|GetDoorName) (Variables|/Game/DEV/Taylor/GameInstance/GI_SpawnPoints.GI_SpawnPoints_C|GetSpawn _asgi_spawn_points))
    (Transformation|Teleport (Game|GetPlayerCharacter 0) (Transformation|GetWorldLocation (Variables|Default|GetArrow)) "0, 0, 0")))

(event Collision|EventActorBeginOverlap
  (params (OtherActor :type Actor%20Object%20Reference)))

(event EventTick
  (params (DeltaSeconds :type Float%20%28single-precision%29)))

(fn ConstructionScript)

(fn OverlayFadein
  (CameraFades|StartCameraFade :self (Game|GetPlayerCameraManager 0) :ToAlpha 1.5 :Duration 0.5 :bHoldWhenFinished true))