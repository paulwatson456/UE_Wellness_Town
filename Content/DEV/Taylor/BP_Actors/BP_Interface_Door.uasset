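; Interactable level-transition door that travels to the level named in its LevelName variable when it receives GeneralInteract.
; It has BP_TP_InterfaceExample fade out the camera, then waits briefly before opening that level.
; When leaving the InyerfaceExample level, it first replaces the DoorPos save slot with a new DoorPosition save holding its Arrow's world location.
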(event EventBeginPlay)

(event Collision|EventActorBeginOverlap
  (params (OtherActor :type Actor%20Object%20Reference)))

(event EventTick
  (params (DeltaSeconds :type Float%20%28single-precision%29)))

(event EventGeneralInteract
  (bind _returnvalue (Actor|GetActorOfClass "/Game/DEV/Taylor/BP_CC/BP_TP_InterfaceExample.BP_TP_InterfaceExample_C"))
  (Default|CameraFadeOut _returnvalue)
  (Utilities|FlowControl|Delay 1.25)
  (bind _returnvalue_2 (Game|GetCurrentLevelName true))
  (if (Utilities|Enum|Equal(Enum) _returnvalue_2 "InyerfaceExample")
    (SaveGame|DeleteGameinSlot "DoorPos")
    (bind _returnvalue_3 (SaveGame|CreateSaveGameObject "/Game/DEV/Taylor/BP_CC/DoorPosition.DoorPosition_C"))
    (Variables|/Game/DEV/Taylor/BP_CC/DoorPosition.DoorPosition_C|SetDoorLocatiion _returnvalue_3 (Transformation|GetWorldLocation (Variables|Default|GetArrow)))
    (SaveGame|SaveGametoSlot _returnvalue_3 "DoorPos"))
  (Game|OpenLevel(byName) (Variables|Default|GetLevelName)))

(fn ConstructionScript)