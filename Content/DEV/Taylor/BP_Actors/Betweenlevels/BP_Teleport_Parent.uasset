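; Parent Blueprint for teleport doors that move the player between levels and place them at the matching door on arrival.
; SetSpawnPos fades the camera, waits, saves DoorName as Spawn in GI_WellnessTown, then opens LevelName.
; On BeginPlay, the door whose DoorName matches the saved Spawn teleports the player to its Arrow with zero rotation.
; The construction script positions that Arrow from SpawnPointOffsetArrow.
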(event Custom|SetSpawnPos
  (CallFunction|OverlayFadein)
  (Utilities|FlowControl|Delay (Variables|Default|GetOpenLevelDelay))
  (bind _asgi_wellness_town (Utilities|Casting|CastToGI_WellnessTown (Game|GetGameInstance)))
  (Variables|/Game/DEV/Taylor/GameInstance/GI_WellnessTown.GI_WellnessTown_C|SetSpawn _asgi_wellness_town (Variables|Default|GetDoorName))
  (Game|OpenLevel(byName) (Variables|Default|GetLevelName)))

(event EventBeginPlay
  (bind _asgi_wellness_town (Utilities|Casting|CastToGI_WellnessTown (Game|GetGameInstance)))
  (if (Utilities|Enum|Equal(Enum) (Variables|Default|GetDoorName) (Variables|/Game/DEV/Taylor/GameInstance/GI_WellnessTown.GI_WellnessTown_C|GetSpawn _asgi_wellness_town))
    (Transformation|Teleport (Game|GetPlayerCharacter 0) (Transformation|GetWorldLocation (Variables|Default|GetArrow)) "0, 0, 0")))

(fn ConstructionScript
  (Transformation|SetRelativeLocation (Variables|Default|GetArrow) (Variables|Default|GetSpawnPointOffset%28Arrow%29) false false))

(fn OverlayFadein
  (CameraFades|StartCameraFade :self (Game|GetPlayerCameraManager 0) :ToAlpha (Variables|Default|GetFade_Alpha) :Duration (Variables|Default|GetFade_Duration) :bHoldWhenFinished true))