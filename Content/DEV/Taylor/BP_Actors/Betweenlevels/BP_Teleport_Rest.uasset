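; Rest arrival point between levels that presents a reflection widget when the game instance's Spawn matches its DoorName.
; On BeginPlay it blends the camera to itself, disables player input, shows the cursor and advances "Rest" progress for objectives of a matching type.
; A timeline then fades in the widget, with a helper rebuilding the border brush to animate outline alpha.
; The Finished event reverses that timeline to fade it out.
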(event Custom|Finished
  (bind _newtrack_0 (Timeline|SetVisibility Reverse)
    (:Update
      (Widget|SetRenderOpacity (stale EventBeginPlay _aswi_reflect_widget) _newtrack_0)
      (CallFunction|SetOutlineOpacity (Variables|/Game/DEV/Taylor/Widgets/WI_ReflectWidget.WI_ReflectWidget_C|GetBorder_0 (stale EventBeginPlay _aswi_reflect_widget)) _newtrack_0))))

(event EventBeginPlay
  (bind _returnvalue (Game|GetPlayerController 0))
  (|CallParentFunction)
  (bind _asgi_wellness_town (Utilities|Casting|CastToGI_WellnessTown (Game|GetGameInstance)))
  (if (Utilities|Enum|Equal(Enum) (Variables|/Game/DEV/Taylor/GameInstance/GI_WellnessTown.GI_WellnessTown_C|GetSpawn _asgi_wellness_town) (Variables|Default|GetDoorName))
    (Game|Player|SetViewTargetwithBlend (Game|GetPlayerController 0) self 2.0 "VTBlend_Linear" 0.0 false)
    (Input|DisableInput (Game|GetPlayerCharacter 0) _returnvalue)
    (Utilities|FlowControl|Delay 2.0)
    (Variables|/Script/Engine.PlayerController|SetbShowMouseCursor _returnvalue true)
    (bind _objective (Utilities|GetObjective)
      (:output
        (if (Utilities|Enum|Equal(Enum) (.Type (Utilities|Struct|BreakS_ObjectiveDetails _objective)) "NewEnumerator6")
          (bind _asbp_tp_interface_example (Utilities|Casting|CastToBP_TP_InterfaceExample (Game|GetPlayerCharacter 0)))
          (Default|ObjectiveProgress _asbp_tp_interface_example "Rest")))
      (:Completed
        (bind _aswi_reflect_widget (Utilities|Casting|CastToWI_ReflectWidget (UserInterface|GetWidget (Variables|Default|GetWidget))))
        (bind _newtrack_0 (Timeline|SetVisibility Play)
          (:Update
            (Widget|SetRenderOpacity _aswi_reflect_widget _newtrack_0)
            (CallFunction|SetOutlineOpacity (Variables|/Game/DEV/Taylor/Widgets/WI_ReflectWidget.WI_ReflectWidget_C|GetBorder_0 _aswi_reflect_widget) _newtrack_0)))))))

(event Collision|EventActorBeginOverlap
  (params (OtherActor :type Actor%20Object%20Reference)))

(event EventTick
  (params (DeltaSeconds :type Float%20%28single-precision%29)))

(fn ConstructionScript
  (|CallParentFunction))

(fn SetOutlineOpacity
  (params (Outline :type Border%20Object%20Reference) (Opacity :type Float%20%28double-precision%29))
  (bind _background (Variables|/Script/UMG.Border|GetBackground Outline))
  (Class|Border|SetBrush Outline (Utilities|Struct|MakeSlateBrush (.drawas _background) (.tiling _background) (.mirroring _background) (.imagesize _background) (.margin _background) (.tintcolor _background) (Utilities|Struct|MakeSlateBrushOutlineSettings (.cornerradii (.outlinesettings _background)) (Utilities|Struct|MakeSlateColor (Utilities|Struct|MakeLinearColor (.r (.specifiedcolor (.color (.outlinesettings _background)))) (.g (.specifiedcolor (.color (.outlinesettings _background)))) (.b (.specifiedcolor (.color (.outlinesettings _background)))) Opacity) (.coloruserule (.color (.outlinesettings _background)))) (.width (.outlinesettings _background)) (.roundingtype (.outlinesettings _background)) (.busebrushtransparency (.outlinesettings _background))) (.resourceobject _background))))