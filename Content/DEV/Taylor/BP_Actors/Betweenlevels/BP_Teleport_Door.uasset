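; Interactable door, apparently for travel between levels, that animates the player's approach and swings open.
; On interact it disables the prompt and input, lerps the player toward an arrow while facing the door, plays the open timeline, then calls SetSpawnPos after a short delay.
; On BeginPlay, if the game instance's Spawn matches DoorName, it reverses that timeline to swing shut behind the arrival, with a delayed close sound.
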(event Custom|OpenDoor
  (Audio|PlaySoundatLocation (Variables|Default|GetSound_DoorOpen) "0, 0, 0" "0, 0, 0" 1.0 1.0 0.0 0 0 0 0)
  (bind _newtrack_0 (Timeline|Timeline Play)
    (:Update
      (if (Variables|Default|GetFlipRotation)
        (Transformation|SetRelativeRotation (Variables|Default|GetPivot) (Math|Rotator|MakeRotator 0.0 0.0 _newtrack_0) false false)
        (else
          (Transformation|SetRelativeRotation (Variables|Default|GetPivot) (Math|Rotator|MakeRotator 0.0 0.0 (* _newtrack_0 -1.0)) false false))))))

(event Custom|CloseDoor
  (Utilities|FlowControl|Sequence
    (:then_0
      (bind _newtrack_0 (Timeline|Timeline ReverseFromEnd)
        (:Update
          (if (Variables|Default|GetFlipRotation)
            (Transformation|SetRelativeRotation (Variables|Default|GetPivot) (Math|Rotator|MakeRotator 0.0 0.0 _newtrack_0) false false)
            (else
              (Transformation|SetRelativeRotation (Variables|Default|GetPivot) (Math|Rotator|MakeRotator 0.0 0.0 (* _newtrack_0 -1.0)) false false))))))
    (:then_1
      (Utilities|FlowControl|Delay 0.7)
      (Audio|PlaySoundatLocation (Variables|Default|GetSound_DoorClose) "0, 0, 0" "0, 0, 0" 1.0 1.0 0.0 0 0 0 0))))

(event Custom|MovePlayer
  (bind _asbp_tp_interface_example (Utilities|Casting|CastToBP_TP_InterfaceExample (Game|GetPlayerCharacter 0)))
  (Input|DisableInput _asbp_tp_interface_example (Game|GetPlayerController 0))
  (bind _newtrack_0 (Timeline|Timeline_0 Play)
    (:Update
      (Transformation|SetWorldLocation (Variables|/Script/Engine.Character|GetCapsuleComponent _asbp_tp_interface_example) (Math|Vector|MakeVector (.x (Math|Vector|Lerp(Vector) (Transformation|GetWorldLocation (Variables|/Script/Engine.Character|GetCapsuleComponent _asbp_tp_interface_example)) (Transformation|GetWorldLocation (Variables|Default|GetArrow)) _newtrack_0)) (.y (Math|Vector|Lerp(Vector) (Transformation|GetWorldLocation (Variables|/Script/Engine.Character|GetCapsuleComponent _asbp_tp_interface_example)) (Transformation|GetWorldLocation (Variables|Default|GetArrow)) _newtrack_0)) (.Z (Math|Vector|BreakVector (Transformation|GetWorldLocation (Variables|/Script/Engine.Character|GetCapsuleComponent _asbp_tp_interface_example))))) false false)
      (Transformation|SetWorldRotation (Variables|/Script/Engine.Character|GetCapsuleComponent _asbp_tp_interface_example) (Math|Rotator|MakeRotator 0.0 0.0 (.yaw (Math|Rotator|FindLookatRotation (Transformation|GetWorldLocation (Variables|/Script/Engine.Character|GetCapsuleComponent _asbp_tp_interface_example)) (Transformation|GetWorldLocation (Variables|Default|GetDoor))))) false false))))

(event EventBeginPlay
  (|CallParentFunction)
  (bind _asgi_wellness_town (Utilities|Casting|CastToGI_WellnessTown (Game|GetGameInstance)))
  (if (Utilities|Enum|Equal(Enum) (Variables|/Game/DEV/Taylor/GameInstance/GI_WellnessTown.GI_WellnessTown_C|GetSpawn _asgi_wellness_town) (Variables|Default|GetDoorName))
    (CallFunction|CloseDoor)))

(event Collision|EventActorBeginOverlap
  (params (OtherActor :type Actor%20Object%20Reference)))

(event EventTick
  (params (DeltaSeconds :type Float%20%28single-precision%29)))

(event EventGeneralInteract
  (bind _asbp_interact_prompt (Utilities|Casting|CastToBP_InteractPrompt (Variables|/Script/Engine.ChildActorComponent|GetChildActor (Variables|Default|GetBP_InteractPrompt))))
  (Variables|/Game/DEV/Taylor/BP_Actors/BP_InteractPrompt.BP_InteractPrompt_C|SetCanInteract? _asbp_interact_prompt false)
  (CallFunction|MovePlayer)
  (CallFunction|OpenDoor)
  (Utilities|FlowControl|Delay 0.5)
  (CallFunction|SetSpawnPos))

(event EventShowPrompt
  (bind _asbp_interact_prompt (Utilities|Casting|CastToBP_InteractPrompt (Variables|/Script/Engine.ChildActorComponent|GetChildActor (Variables|Default|GetBP_InteractPrompt))))
  (Default|ShowPrompt _asbp_interact_prompt))

(fn ConstructionScript
  (|CallParentFunction))