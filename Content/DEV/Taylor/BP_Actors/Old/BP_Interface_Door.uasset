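; Interactable level-transition door that links levels and places the arriving player at the matching door.
; On interact, it swings open via a timeline with an optional flipped direction, fades the camera, saves the current level name to a DoorPosition slot and opens its target level.
; On BeginPlay, a door whose target matches the saved level teleports the player to its arrow, clears the save and animates closed.
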(event Custom|OpenDoor
  (bind _newtrack_0 (Timeline|DoorAnimations Play)
    (:Update
      (if (Variables|Default|GetFlipRotation)
        (Transformation|SetRelativeRotation (Variables|Default|GetPivot) (Math|Rotator|MakeRotator 0.0 0.0 _newtrack_0) false false)
        (else
          (Transformation|SetRelativeRotation (Variables|Default|GetPivot) (Math|Rotator|MakeRotator 0.0 0.0 (* _newtrack_0 -1.0)) false false))))))

(event Custom|CloseDoor
  (bind _newtrack_0 (Timeline|DoorAnimations ReverseFromEnd)
    (:Update
      (if (Variables|Default|GetFlipRotation)
        (Transformation|SetRelativeRotation (Variables|Default|GetPivot) (Math|Rotator|MakeRotator 0.0 0.0 _newtrack_0) false false)
        (else
          (Transformation|SetRelativeRotation (Variables|Default|GetPivot) (Math|Rotator|MakeRotator 0.0 0.0 (* _newtrack_0 -1.0)) false false))))))

(event EventBeginPlay
  (bind _returnvalue (SaveGame|DoesSaveGameExist "DoorPos"))
  (if _returnvalue
    (bind _returnvalue_2 (SaveGame|LoadGamefromSlot "DoorPos"))
    (bind _asdoor_position (Utilities|Casting|CastToDoorPosition _returnvalue_2))
    (if (== (Variables|/Game/DEV/Taylor/BP_CC/DoorPosition.DoorPosition_C|GetLevelName _asdoor_position) (Variables|Default|GetLevelName))
      (Transformation|Teleport (Game|GetPlayerCharacter 0) (Transformation|GetWorldLocation (Variables|Default|GetArrow)) "0, 0, 0")
      (SaveGame|DeleteGameinSlot "DoorPos")
      (CallFunction|CloseDoor))))

(event Collision|EventActorBeginOverlap
  (params (OtherActor :type Actor%20Object%20Reference)))

(event EventTick
  (params (DeltaSeconds :type Float%20%28single-precision%29)))

(event EventGeneralInteract
  (CallFunction|OpenDoor)
  (Utilities|FlowControl|Delay 0.5)
  (Actor|GetActorOfClass "/Game/DEV/Taylor/BP_CC/BP_TP_InterfaceExample.BP_TP_InterfaceExample_C")
  (CallFunction|OverlayFadein)
  (Utilities|FlowControl|Delay 1.25)
  (SaveGame|DeleteGameinSlot "DoorPos")
  (bind _returnvalue (SaveGame|CreateSaveGameObject "/Game/DEV/Taylor/BP_CC/DoorPosition.DoorPosition_C"))
  (bind _returnvalue_2 (Game|GetCurrentLevelName true))
  (Variables|/Game/DEV/Taylor/BP_CC/DoorPosition.DoorPosition_C|SetLevelName _returnvalue (Utilities|String|StringToName _returnvalue_2))
  (SaveGame|SaveGametoSlot _returnvalue "DoorPos")
  (Game|OpenLevel(byName) (Variables|Default|GetLevelName)))

(fn ConstructionScript)

(fn OverlayFadein
  (CameraFades|StartCameraFade :self (Game|GetPlayerCameraManager 0) :ToAlpha 1.5 :Duration 1.0 :bHoldWhenFinished true))