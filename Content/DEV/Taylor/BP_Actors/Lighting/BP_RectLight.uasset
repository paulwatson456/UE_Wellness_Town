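; Configurable rect light actor with a daytime setup and an enabled lighting state that can flicker.
; The construction script applies the day temperature and intensities, light shape, attenuation radius and initial visibility from variables.
; LightingEnable shows the actor's components, turns on shadows, sets indirect intensity and randomizes brightness and temperature around Intensity and Warmth.
; With Flicker on, that randomization repeats in an endless loop at short random delays.
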(event EventLightingEnable
  (bind _rectlight (Variables|Default|GetRectLight))
  (bind _warmth (Variables|Default|GetWarmth))
  (bind _intensity (Variables|Default|GetIntensity))
  (bind _rectlight_2 (Variables|Default|GetRectLight))
  (bind _rectlight_3 (Variables|Default|GetRectLight))
  (bind _warmth_2 (Variables|Default|GetWarmth))
  (bind _intensity_2 (Variables|Default|GetIntensity))
  (Rendering|SetVisibility (Variables|Default|GetDefaultSceneRoot) true true)
  (Rendering|Components|Light|SetCastShadows _rectlight_3 true)
  (Class|LightComponent|SetIndirectLightingIntensity _rectlight_3 (Variables|Default|GetIndirectLightingIntensity))
  (if (Variables|Default|GetFlicker?)
    (Rendering|Components|Light|SetIntensity _rectlight_2 (Math|Random|RandomFloatinRange (- _intensity 1e+03) (+ _intensity 1e+03)) :!label _label)
    (Class|LightComponent|SetTemperature _rectlight_2 (Math|Random|RandomFloatinRange (- _warmth 1.5e+02) (+ _warmth 1.5e+02)))
    (Utilities|FlowControl|Delay (Math|Random|RandomFloatinRange 0.05 0.2))
    (goto _label)
    (else
      (Rendering|Components|Light|SetIntensity _rectlight (Math|Random|RandomFloatinRange (- _intensity_2 1e+03) (+ _intensity_2 1e+03)))
      (Class|LightComponent|SetTemperature _rectlight (Math|Random|RandomFloatinRange (- _warmth_2 1.5e+02) (+ _warmth_2 1.5e+02))))))

(fn ConstructionScript
  (bind _rectlight (Variables|Default|GetRectLight))
  (bind _rectlight_2 (Variables|Default|GetRectLight))
  (Class|LightComponent|SetTemperature _rectlight (Variables|Default|GetDayTemp))
  (Rendering|Components|Light|SetIntensity _rectlight (Variables|Default|GetDayInt))
  (Class|RectLightComponent|SetBarnDoorAngle _rectlight (Variables|Default|GetAngle))
  (Class|RectLightComponent|SetSourceHeight _rectlight (Variables|Default|Getheight))
  (Class|RectLightComponent|SetSourceWidth _rectlight (Variables|Default|GetWidth))
  (Class|LightComponent|SetIndirectLightingIntensity _rectlight_2 (Variables|Default|GetDayIndirectInt))
  (Rendering|Lighting|SetAttenuationRadius _rectlight_2 (Variables|Default|GetAttenuationRadius))
  (Rendering|SetVisibility (Variables|Default|GetDefaultSceneRoot) (Variables|Default|GetVisible?) true))